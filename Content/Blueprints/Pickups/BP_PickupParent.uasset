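; Parent pickup Blueprint for reagents that the player collects by touching them, with gravity enabled on its Box at BeginPlay.
; When the BP_PlayerGuy capsule overlaps the Box, PickUpIndex selects which of seven reagent counters on the player to increment.
; It then hides the Billboard, disables overlaps, plays a WB_PopUp "+ 1" name popup and destroys itself.
; Unconnected ReagentMap and Delay nodes never run.
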(event OnComponentBeginOverlap(Box)
  (params (OverlappedComponent :type Primitive%20Component%20Object%20Reference) (OtherActor :type Actor%20Object%20Reference) (OtherComp :type Primitive%20Component%20Object%20Reference) (OtherBodyIndex :type Integer) (bFromSweep :type Boolean) (SweepResult :type Hit%20Result%20Structure%20%28by%20ref%29))
  (bind _asbp_player_guy (Utilities|Casting|CastToBP_PlayerGuy OtherActor))
  (if (== OtherComp (Variables|/Script/Engine.Character|GetCapsuleComponent _asbp_player_guy))
    (switch int (Variables|Default|GetPickUpIndex)
      (:1
        (bind _result (Math|Integer|IncrementInt (Variables|/Game/Blueprints/BP_PlayerGuy.BP_PlayerGuy_C|GetReagent%20Mushroom _asbp_player_guy))
          (:%20%20
            (Variables|/Game/Blueprints/BP_PlayerGuy.BP_PlayerGuy_C|SetReagent%20Mushroom _asbp_player_guy _result))))
      (:2
        (bind _result_2 (Math|Integer|IncrementInt (Variables|/Game/Blueprints/BP_PlayerGuy.BP_PlayerGuy_C|GetReagent%20Crystal _asbp_player_guy))
          (:%20%20
            (Variables|/Game/Blueprints/BP_PlayerGuy.BP_PlayerGuy_C|SetReagent%20Crystal _asbp_player_guy _result_2))))
      (:3
        (bind _result_3 (Math|Integer|IncrementInt (Variables|/Game/Blueprints/BP_PlayerGuy.BP_PlayerGuy_C|GetReagent%20Herb _asbp_player_guy))
          (:%20%20
            (Variables|/Game/Blueprints/BP_PlayerGuy.BP_PlayerGuy_C|SetReagent%20Herb _asbp_player_guy _result_3))))
      (:4
        (bind _result_4 (Math|Integer|IncrementInt (Variables|/Game/Blueprints/BP_PlayerGuy.BP_PlayerGuy_C|GetReagent%20Eye _asbp_player_guy))
          (:%20%20
            (Variables|/Game/Blueprints/BP_PlayerGuy.BP_PlayerGuy_C|SetReagent%20Eye _asbp_player_guy _result_4))))
      (:5
        (bind _result_5 (Math|Integer|IncrementInt (Variables|/Game/Blueprints/BP_PlayerGuy.BP_PlayerGuy_C|GetReagent%20Flower _asbp_player_guy))
          (:%20%20
            (Variables|/Game/Blueprints/BP_PlayerGuy.BP_PlayerGuy_C|SetReagent%20Flower _asbp_player_guy _result_5))))
      (:6
        (bind _result_6 (Math|Integer|IncrementInt (Variables|/Game/Blueprints/BP_PlayerGuy.BP_PlayerGuy_C|GetReagent%20Heart _asbp_player_guy))
          (:%20%20
            (Variables|/Game/Blueprints/BP_PlayerGuy.BP_PlayerGuy_C|SetReagent%20Heart _asbp_player_guy _result_6))))
      (:7
        (bind _result_7 (Math|Integer|IncrementInt (Variables|/Game/Blueprints/BP_PlayerGuy.BP_PlayerGuy_C|GetReagent%20Moth _asbp_player_guy))
          (:%20%20
            (Variables|/Game/Blueprints/BP_PlayerGuy.BP_PlayerGuy_C|SetReagent%20Moth _asbp_player_guy _result_7)))))
    (Rendering|SetVisibility (Variables|Default|GetBillboard) false true)
    (Variables|/Script/Engine.PrimitiveComponent|SetbGenerateOverlapEvents (Variables|Default|GetBox) false)
    (bind _returnvalue (UserInterface|CreateWidget "/Game/Blueprints/UI/WB_PopUp.WB_PopUp_C" 0 self 2.0 (Utilities|String|Append "+ 1 " (Variables|Default|GetName))))
    (UserInterface|Viewport|AddtoViewport _returnvalue 0)
    (UserInterface|Animation|PlayAnimation _returnvalue (Variables|/Game/Blueprints/UI/WB_PopUp.WB_PopUp_C|GetPopUpAnimation _returnvalue) 0.0 1 "Forward" 1.0 false)
    (Actor|DestroyActor)))

(event EventBeginPlay
  (Physics|SetEnableGravity (Variables|Default|GetBox) true))

(event Collision|EventActorBeginOverlap
  (params (OtherActor :type Actor%20Object%20Reference)))

(event EventTick
  (params (DeltaSeconds :type Float%20%28single-precision%29)))

(fn ConstructionScript)